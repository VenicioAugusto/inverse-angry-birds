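; Player camera controller that pans the view by mouse drag and lets the player grab and drag objects under the cursor.
; Camera drag offsets the actor in X and Z by the viewport mouse delta while right mouse is held, unless grabbing.
; Object drag line-traces from the cursor and stores hit distance and grab offset for movable components.
; Tick follows the deprojected cursor at that distance, using a PhysicsHandle for simulated bodies, otherwise SetWorldLocation.
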(event EventBeginPlay
  (bind _returnvalue (Game|GetPlayerController 0))
  (Variables|/Script/Engine.PlayerController|SetbShowMouseCursor _returnvalue true)
  (Variables|/Script/Engine.PlayerController|SetbEnableTouchEvents _returnvalue true))

(event EventTick
  (params (DeltaSeconds :type Float%20%28single-precision%29))
  (bind _returnvalue (Game|GetPlayerController 0))
  (bind _originaldistancetoobject (Variables|Default|GetOriginalDistanceToObject))
  (bind (_worldlocation _worlddirection) (Game|Player|ConvertMouseLocationToWorldSpace _returnvalue))
  (bind _returnvalue_2 (* _worlddirection _originaldistancetoobject))
  (bind _returnvalue_3 (+ _worldlocation _returnvalue_2))
  (if (not (Variables|Default|GetIsGrabbing))
    (if (Variables|Default|GetIsMovingCamera)
      ;[1 1 1] CameraMovement
      (if (Game|Player|IsInputKeyDown (Game|GetPlayerController 0) "RightMouseButton")
        (bind _returnvalue_4 (Class|WidgetLayoutLibrary|GetMousePositiononViewport))
        (Variables|Default|SetNew%20Location _returnvalue_4)
        (Transformation|AddActorWorldOffset (Math|Vector|MakeVector (.x (- (Variables|Default|GetNew%20Location) (Variables|Default|GetPreviews%20Location))) 0.0 (.y (- (Variables|Default|GetNew%20Location) (Variables|Default|GetPreviews%20Location)))))
        (Variables|Default|SetPreviews%20Location (Variables|Default|GetNew%20Location))))
    (else
      ;[1 1 1] Object Movement
      (if (Physics|IsSimulatingPhysics (Variables|Default|GetGrabbedObject) "None")
        (Physics|Components|PhysicsHandle|SetTargetLocation (Variables|Default|GetPhysicsHandle) _returnvalue_3)
        (else
          (Transformation|SetWorldLocation (Variables|Default|GetGrabbedObject) (Math|Transform|InverseTransformLocation (Math|Conversions|ToTransform(Vector) (Variables|Default|GetRelativeGrabLocation)) _returnvalue_3) false false))))))

(event Input|ActionEvents|InputActionDragCamera
  (params (Key :type Key%20Structure :default "None"))
  (:Pressed
    (if (not (Variables|Default|GetIsGrabbing))
      (Variables|Default|SetIsMovingCamera true)
      (bind _returnvalue (Class|WidgetLayoutLibrary|GetMousePositiononViewport))
      (Variables|Default|SetPreviews%20Location _returnvalue)))
  (:Released
    (Variables|Default|SetIsMovingCamera false)))

(event Input|ActionEvents|InputActionDragObjects
  (params (Key :type Key%20Structure :default "None"))
  (bind _returnvalue (Game|GetPlayerController 0))
  (bind (_worldlocation _worlddirection) (Game|Player|ConvertMouseLocationToWorldSpace _returnvalue))
  (:Pressed
    (bind _returnvalue_2 (Class|WidgetLayoutLibrary|GetMousePositiononViewport))
    (Variables|Default|SetPreviews%20Location _returnvalue_2)
    (bind (_outhit _returnvalue_3) (Collision|LineTraceByChannel _worldlocation (+ _worldlocation (* _worlddirection (Math|Float|MakeLiteralFloat 1e+03))) "TraceTypeQuery3" false 0 "ForDuration"))
    (if _returnvalue_3
      (Variables|Default|SetIsGrabbing true)
      (Variables|Default|SetRelativeGrabLocation (Math|Transform|InverseTransformLocation (Math|Conversions|ToTransform(Vector) (Transformation|GetWorldLocation (.HitComponent (Collision|BreakHitResult _outhit)))) (.Location (Collision|BreakHitResult _outhit))))
      (Variables|Default|SetOriginalDistanceToObject (.Distance (Collision|BreakHitResult _outhit)))
      (if (Utilities|Enum|Equal(Enum) (Variables|/Script/Engine.SceneComponent|GetMobility (.HitComponent (Collision|BreakHitResult _outhit))) "Movable")
        (bind _output_get (Variables|Default|SetGrabbedObject (.HitComponent (Collision|BreakHitResult _outhit))))
        (Class|PhysicsHandleComponent|GrabComponentatLocation (Variables|Default|GetPhysicsHandle) _output_get "None" (Transformation|GetWorldLocation _output_get)))))
  (:Released
    (Variables|Default|SetIsGrabbing false)
    (Variables|Default|SetGrabbedObject 0)
    (Physics|Components|PhysicsHandle|ReleaseComponent (Variables|Default|GetPhysicsHandle))))

(fn ConstructionScript)