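; Game manager actor that runs a building game, switching between Construction Mode and a physics-driven Action Mode.
; On BeginPlay it caches controller, camera, HUD and map-variables actors, copies the map's material budget and enters Construction Mode.
; It spawns materials at a camera offset, forwards rotation to the camera controller, and reports or resets quantities.
; Action Mode enables physics on every material actor's meshes; level reset destroys those actors by class.
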(event Custom|ToActionMode
  ;[1 1 1] Activate Action Mode
  (for _array_element (Variables|/Game/Blueprints/BP_Map_Variables.BP_Map_Variables_C|GetAllDiferentMaterials (Variables|Default|GetMap%20Materials%20Ref))
    (bind _outactors (Actor|GetAllActorsOfClass _array_element))
    (for _array_element_2 _outactors
      (for _array_element_3 (Actor|GetComponentsByClass _array_element_2 "/Script/Engine.StaticMeshComponent")
        (Physics|SetSimulatePhysics _array_element_3 true)
        (Class|PrimitiveComponent|SetConstraintMode _array_element_3 "Default"))
      (Default|SetActionModeCC (Variables|Default|GetBP_CameraControllerRef) true))))

(event Custom|ResetMaterialsQuantity
  ;[1 1 1] Reset Materials Quantity
  (Variables|Default|SetBuild%20Materials%20from%20Map (Variables|Default|GetDefault%20Build%20Materials)))

(event Custom|ToConstructionMode
  ;[1 1 1] Activate Construction Mode
  (Default|ActivateConstructionMode (Variables|Default|GetBP_HUDRef))
  (Default|SetActionModeCC (Variables|Default|GetBP_CameraControllerRef) false))

(event Custom|SpawnMaterial
  (params (MaterialToSpawn :type Integer))
  (bind _playerref (Variables|Default|GetPlayerRef))
  (bind _playercameramanager (Variables|/Script/Engine.PlayerController|GetPlayerCameraManager _playerref))
  (bind _returnvalue (Camera|GetCameraLocation _playercameramanager))
  ;[1 1 1] Spawn Material
  (switch int MaterialToSpawn
    (:0
      (Variables|Default|SetMaterialToSpawn (Variables|/Game/Blueprints/BP_Map_Variables.BP_Map_Variables_C|GetMaterial01 (Variables|Default|GetMap%20Materials%20Ref))))
    (:1
      (Variables|Default|SetMaterialToSpawn (Variables|/Game/Blueprints/BP_Map_Variables.BP_Map_Variables_C|GetMaterial02 (Variables|Default|GetMap%20Materials%20Ref)))))
  (Game|SpawnActorfromClass (Variables|Default|GetMaterialToSpawn) (Math|Conversions|ToTransform(Vector) (Math|Vector|MakeVector (.x _returnvalue) (+ (.y _returnvalue) 5e+02) (.z _returnvalue))) "Undefined" "MultiplyWithRoot" 0 0))

(event Custom|ResetLevel
  ;[1 1 1] Reset Level Materials
  (for _array_element (Variables|/Game/Blueprints/BP_Map_Variables.BP_Map_Variables_C|GetAllDiferentMaterials (Variables|Default|GetMap%20Materials%20Ref))
    (bind _outactors (Actor|GetAllActorsOfClass _array_element))
    (Actor|DestroyActor _outactors)))

(event Custom|RotateToDirection
  (params (Direction :type Boolean))
  (Default|RotateObject (Variables|Default|GetBP_CameraControllerRef) Direction))

(event EventBeginPlay
  (bind _returnvalue (Actor|GetActorOfClass "/Game/Player/BP_PlayerController.BP_PlayerController_C"))
  (Variables|Default|SetPlayerRef _returnvalue)
  (bind _returnvalue_2 (Actor|GetActorOfClass "/Game/Player/BP_CameraController.BP_CameraController_C"))
  (Variables|Default|SetBP_CameraControllerRef _returnvalue_2)
  ;[1 1 1] Set Material Quantity
  (bind _returnvalue_3 (Actor|GetActorOfClass "/Game/Blueprints/BP_Map_Variables.BP_Map_Variables_C"))
  (bind _output_get (Variables|Default|SetMap%20Materials%20Ref _returnvalue_3))
  (bind _output_get_2 (Variables|Default|SetDefault%20Build%20Materials (Variables|/Game/Blueprints/BP_Map_Variables.BP_Map_Variables_C|GetBuildMaterials _output_get)))
  (Variables|Default|SetBuild%20Materials%20from%20Map _output_get_2)
  ;[1 1 1] Set the Hud Reference and the default material quantity
  (bind _returnvalue_4 (Actor|GetActorOfClass "/Game/Blueprints/BP_HUD.BP_HUD_C"))
  (bind _output_get_3 (Variables|Default|SetBP_HUDRef _returnvalue_4))
  (Default|SetMapVariables _output_get_3)
  (CallFunction|ToConstructionMode))

(event Collision|EventActorBeginOverlap
  (params (OtherActor :type Actor%20Object%20Reference)))

(event EventTick
  (params (DeltaSeconds :type Float%20%28single-precision%29)))

(fn ConstructionScript)

(fn ReturnMaterialQuantity
  (params (Material :type Name))
  (return (.Value (Utilities|Map|Find (Variables|Default|GetBuild%20Materials%20from%20Map) Material))))